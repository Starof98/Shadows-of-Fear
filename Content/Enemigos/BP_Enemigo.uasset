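; Enemy character Blueprint that patrols around its spawn point and performs a melee bear attack montage.
; Patrullar line-traces random nearby ground points and loops AIMoveTo between them.
; PawnSensing raises walk speed, issues a move without a wired target, plays the attack on success, and resumes patrol after a retriggerable delay.
; While attacking, Tick traces three claw socket pairs, calling ApplyDamage once per listed claw, though no damaged actor is wired.
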(event `Patrullar`
  (bind (_ubicacioninicial_x _ubicacioninicial_y) (`KismetMathLibrary.BreakVector` (`self.UbicacionInicial`)))
  (bind _returnvalue (+ (`KismetMathLibrary.RandomFloatInRange` (* (`self.RadioDeMovimiento`) 0.0) (`self.RadioDeMovimiento`)) _ubicacioninicial_y))
  (bind _returnvalue_2 (+ (`KismetMathLibrary.RandomFloatInRange` (* (`self.RadioDeMovimiento`) 0.0) (`self.RadioDeMovimiento`)) _ubicacioninicial_x))
  ;[1 1 1] Patrullar
  (bind _outhit (`KismetSystemLibrary.LineTraceSingle` :`Start` (`KismetMathLibrary.MakeVector` _returnvalue_2 _returnvalue 25000.0) :`End` (`KismetMathLibrary.MakeVector` _returnvalue_2 _returnvalue) :`TraceChannel` "TraceTypeQuery1" :`DrawDebugType` "ForDuration" :`DrawTime` 100.0 :!label _label))
  (`|AIMoveTo` self (`.ImpactPoint` (`GameplayStatics.BreakHitResult` _outhit)) null
    (:`OnSuccess`
      (`KismetSystemLibrary.Delay` 5.0)
      (goto _label))))

(event `self.ReceiveBeginPlay`
  ;[1 1 1] Patrullar
  (set `self.UbicacionInicial` (`self.K2_GetActorLocation`))
  (`self.Patrullar`))

(event `self.PawnSensing.OnSeePawn`
  (params (Pawn :type "Pawn Object Reference"))
  (bind _returnvalue (`AnimInstance.IsAnyMontagePlaying` (`SkeletalMeshComponent.GetAnimInstance` (`self.Mesh`))))
  ;[1 1 1] Sensor de Visión
  (`self.Cambiar velocidad` 350.0)
  (if _returnvalue
    (`KismetSystemLibrary.RetriggerableDelay` 2.0 :!label _label_2)
    (`self.Patrullar`)
    (else
      (`KismetSystemLibrary.PrintString` "Estoy viendo a Adam")
      (`|AIMoveTo` self (0.0 0.0 0.0) null 300.0
        (:`then`
          (goto _label_2))
        (:`OnSuccess`
          (if (not _returnvalue)
            (`KismetSystemLibrary.PrintString` "Atacar")
            (`|PlayMontage` (`self.Mesh`) "/Game/InfinityBladeAdversaries/Enemy/Enemy_Bear/Enemy_Bear_Animations/ExoGame_Bears_Attack_Melee_B_Montage.ExoGame_Bears_Attack_Melee_B_Montage")))))))

(event `self.ReceiveTick`
  (params (DeltaSeconds :type "Float (single-precision)"))
  ;[1 1 1] Ataque
  (if (`self.RealizandoAtaque`)
    (`self.Revisar Danio` "Inicio1" "Final1" 1)
    (`self.Revisar Danio` "Inicio2" "Final2" 2)
    (`self.Revisar Danio` "Inicio3" "Final3" 3)))

(event `Cambiar velocidad`
  (params (Velocidad :type "Float (double-precision)"))
  ;[1 1 1] Cambiar velocidad
  (set `CharacterMovementComponent.MaxWalkSpeed` Velocidad (`self.CharacterMovement`)))

(event `AtaqueIzquierda`)

(event `AtaqueDerecha`)

(event `AtaqueBasico`)

(fn `Revisar Danio`
  (params (Inicio :type Name) (Final :type Name) (Garra :type Integer))
  (bind _mesh (`self.Mesh`))
  (if (not (`KismetArrayLibrary.Array_Contains` (`self.GarrasConDanio`) Garra))
    (bind (_outhit _returnvalue) (`KismetSystemLibrary.LineTraceSingle` :`Start` (`SceneComponent.GetSocketLocation` _mesh Inicio) :`End` (`SceneComponent.GetSocketLocation` _mesh Final) :`TraceChannel` "TraceTypeQuery2" :`DrawDebugType` "ForDuration"))
    (if _returnvalue
      (`GameplayStatics.ApplyDamage` null 8.0 (`self.GetInstigatorController`) self "/Script/Engine.DamageType")
      (`KismetArrayLibrary.Array_Add` (`self.GarrasConDanio`) (`local.Garra`)))))

(fn `UserConstructionScript`)