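; HUD helper object that animates an ammo counter counting up when ammo is added.
; StartAmmoUpdate computes the target total, then after a short delay starts a fast looping timer on UpdateAmmo.
; UpdateAmmo lerps the displayed number toward the target, clearing the timer once it overshoots and showing the final value.
; The pocket ammo text mirrors the count when the current weapon uses the same ammo type.
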(event `StartAmmoUpdate`
  (set `self.EndAmmo` (`KismetMathLibrary.Conv_IntToDouble` (+ (`self.CurrentAmmo`) (`self.+Ammo`))))
  (`KismetSystemLibrary.K2_SetTimerDelegate` (delegate `StartTimerUpdate`) 0.5))

(event `StartTimerUpdate`
  (`KismetSystemLibrary.K2_SetTimer` null "UpdateAmmo" 0.01 true))

(fn `UpdateAmmo`
  (bind _playercurrentweapon (`self.PlayerCurrentWeapon`))
  (bind _playercurrentweapon_2 (`self.PlayerCurrentWeapon`))
  (bind _returnvalue (`KismetTextLibrary.Conv_IntToText` (`KismetMathLibrary.FTrunc` (`self.EndAmmo`))))
  (bind _returnvalue_2 (`KismetMathLibrary.Lerp` (`KismetMathLibrary.Conv_IntToDouble` (`self.CurrentAmmo`)) (`self.EndAmmo`) (/ (`self.ForTimer`) 0.5)))
  (bind _output_get (set `self.CurrentUpdateAmmo` _returnvalue_2))
  (if (> _output_get (`self.EndAmmo`))
    (`KismetSystemLibrary.K2_ClearTimer` null "UpdateAmmo")
    (`TextBlock.SetText` (`self.Ammo`) _returnvalue)
    (`/Engine/EditorBlueprintResources/StandardMacros.IsValid` _playercurrentweapon_2
      (:`Is Valid`
        (if (`KismetStringLibrary.EqualEqual_StrStr` (`.AmmoType_11_9A87780A4682B1D96AF46EBA94369155` (break `/Game/Interaction/Blueprints/Weapon/Structures/Struct_W_Ammo` (`.Ammo_17_29EF0D6441F39BA7FA17B3A328E67A64` (break `/Game/Interaction/Blueprints/Weapon/Structures/Struct_W` (`/Game/Interaction/Blueprints/Weapon/BP_Weapon.WeaponStruct` _playercurrentweapon_2))))) (`self.AmmoTypeName`))
          (`TextBlock.SetText` (`self.AmmoPocket`) _returnvalue))))
    (else
      (`TextBlock.SetText` (`self.Ammo`) (`KismetTextLibrary.Conv_IntToText` (`KismetMathLibrary.FTrunc` _returnvalue_2)))
      (set `self.ForTimer` (+ (`self.ForTimer`) 0.01))
      (`/Engine/EditorBlueprintResources/StandardMacros.IsValid` _playercurrentweapon
        (:`Is Valid`
          (if (`KismetStringLibrary.EqualEqual_StrStr` (`.AmmoType_11_9A87780A4682B1D96AF46EBA94369155` (break `/Game/Interaction/Blueprints/Weapon/Structures/Struct_W_Ammo` (`.Ammo_17_29EF0D6441F39BA7FA17B3A328E67A64` (break `/Game/Interaction/Blueprints/Weapon/Structures/Struct_W` (`/Game/Interaction/Blueprints/Weapon/BP_Weapon.WeaponStruct` _playercurrentweapon))))) (`self.AmmoTypeName`))
            (`TextBlock.SetText` (`self.AmmoPocket`) (`TextBlock.GetText` (`self.Ammo`)))))))))