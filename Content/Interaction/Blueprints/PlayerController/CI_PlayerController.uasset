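; Player controller that handles the weapon manager screen, a custom cursor widget and a demo radial menu.
; The WeaponManager input toggles weapon storage on the pawn's HUD, switching input mode and cursor and disabling pawn input while open.
; Holding key 1 shows DemoWidget and centers the mouse on its panel; release removes it.
; An unconnected calculation derives radial distance and angle from the mouse position.
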(event `InputAction|WeaponManager`
  (params (Key :type "Key Structure"))
  (bind _returnvalue (`GameplayStatics.GetPlayerPawn` 0))
  (:`Pressed`
    (cast `/Game/Interaction/Blueprints/Pawn/Player/Character_Pawn` _returnvalue
      (:`then`
        _)
      (:`CastFailed`
        (cast `/Game/Interaction/Blueprints/Pawn/Player/Character_Pawn_FPS` _returnvalue)))
    (`self.WeaponManager` (not (`self.WeaponManagerActive`)))))

(event `WeaponManager`
  (params (Open :type Boolean))
  (if Open
    (if (not (`self.WeaponManagerActive`))
      (set `self.bShowMouseCursor` true)
      (`WidgetBlueprintLibrary.SetInputMode_GameAndUIEx` self null "DoNotLock" false)
      (`self.DisableInput` (`GameplayStatics.GetPlayerPawn` 0) self)
      (bind _hud (message `/Game/Interaction/Blueprints/Pawn/Player/StatusInterface.GetComponents` (`GameplayStatics.GetPlayerPawn` 0)))
      (`/Game/Interaction/Hud/Hud_WeaponManager.OpenWeaponStorage` (`/Game/Interaction/Hud/HUD_Widget.WeaponManager` _hud) true)
      (set `self.WeaponManagerActive` true))
    (elif (`self.WeaponManagerActive`)
      (set `self.bShowMouseCursor` false)
      (`WidgetBlueprintLibrary.SetInputMode_GameOnly` self)
      (`self.EnableInput` (`GameplayStatics.GetPlayerPawn` 0) self)
      (bind _hud_2 (message `/Game/Interaction/Blueprints/Pawn/Player/StatusInterface.GetComponents` (`GameplayStatics.GetPlayerPawn` 0)))
      (`/Game/Interaction/Hud/Hud_WeaponManager.OpenWeaponStorage` (`/Game/Interaction/Hud/HUD_Widget.WeaponManager` _hud_2) false)
      (set `self.WeaponManagerActive` false))))

(event `self.ReceiveBeginPlay`
  (bind _returnvalue (`|CreateWidget` "/Game/Interaction/Hud/Hud_MouseCursor.Hud_MouseCursor_C"))
  (set `self.CursorWidjet` _returnvalue)
  (`self.SetMouseCursorWidget` "Default" _returnvalue))

(event `Key|One`
  (params (Key :type "Key Structure"))
  (bind _returnvalue (`WidgetLayoutLibrary.GetViewportScale`))
  (bind _returnvalue_2 (`WidgetLayoutLibrary.GetViewportScale`))
  ;[1 1 1] Radial Menu (1)
  (:`Pressed`
    (bind _returnvalue_3 (`|CreateWidget` "/Game/David_Programmer/Radial_Menu/DemoWidget.DemoWidget_C"))
    (`UserWidget.AddToViewport` _returnvalue_3 0)
    (set `self.bShowMouseCursor` true)
    (bind _returnvalue_4 (`WidgetLayoutLibrary.SlotAsCanvasSlot` (`/Game/David_Programmer/Radial_Menu/DemoWidget.CanvasPanel_129` _returnvalue_3)))
    (bind (_x _y) (`KismetMathLibrary.BreakVector2D` (`CanvasPanelSlot.GetPosition` _returnvalue_4)))
    (bind (_x_2 _y_2) (`KismetMathLibrary.BreakVector2D` (`CanvasPanelSlot.GetSize` _returnvalue_4)))
    (`self.SetMouseLocation` (`KismetMathLibrary.FTrunc` (+ (* _x _returnvalue) (/ (* _x_2 _returnvalue_2) 2.0))) (`KismetMathLibrary.FTrunc` (+ (* _y _returnvalue) (/ (* _y_2 _returnvalue_2) 2.0)))))
  (:`Released`
    (bind _foundwidgets (`WidgetBlueprintLibrary.GetAllWidgetsOfClass` "/Game/David_Programmer/Radial_Menu/DemoWidget.DemoWidget_C"))
    (`Widget.RemoveFromParent` (`|GetArrayItem` _foundwidgets))
    (set `self.bShowMouseCursor` false)))

(fn `UserConstructionScript`)