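; Player weapon storage component that keeps the parameters of available standard and melee weapons.
; Adding a weapon looks it up by name in a definition list, or takes a custom struct for non-melee, then stores it in a map under an incrementing index.
; That index retrieves stored parameters, and ChangeWeapon uses it to push them into a given weapon component.
; Failed name lookups print a message.
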(fn `AddWeapon`
  (params (WeaponName :type String) (CustomWeapon :type Boolean) (CustomWeaponStruct :type "/Game/Interaction/Blueprints/Weapon/Structures/Struct_W Structure"))
  (returns (PrimaryWeapon :type Boolean) (AvailableWeaponIndex :type Integer))
  (bind (_value _returnvalue) (`BlueprintMapLibrary.Map_Find` (`self.WeaponList`) WeaponName))
  (if CustomWeapon
    (`/Engine/EditorBlueprintResources/StandardMacros.IncrementInt` (`self.CurrentWeaponIndex`)
      (:`  `
        (`BlueprintMapLibrary.Map_Add` (`self.AvailableWeapons`) (`self.CurrentWeaponIndex`) CustomWeaponStruct)
        (return (`.PrimaryWeapon_28_D758820444D96D64DE568582361A11F7` (break `/Game/Interaction/Blueprints/Weapon/Structures/Struct_W` CustomWeaponStruct)) (`self.CurrentWeaponIndex`))))
    (elif _returnvalue
      (`/Engine/EditorBlueprintResources/StandardMacros.IncrementInt` (`self.CurrentWeaponIndex`)
        (:`  `
          (`BlueprintMapLibrary.Map_Add` (`self.AvailableWeapons`) (`self.CurrentWeaponIndex`) _value)
          (return (`.PrimaryWeapon_28_D758820444D96D64DE568582361A11F7` (break `/Game/Interaction/Blueprints/Weapon/Structures/Struct_W` _value)) (`self.CurrentWeaponIndex`))))
      (else
        (`KismetSystemLibrary.PrintString` "No weapons found (Weapon List). Check the name or add the weapon to the list.")))))

(fn `AddWeaponMelee`
  (params (WeaponName :type String))
  (returns (AvailableWeaponIndex :type Integer))
  (bind (_value _returnvalue) (`BlueprintMapLibrary.Map_Find` (`self.WeaponMeleeList`) WeaponName))
  (if _returnvalue
    (`/Engine/EditorBlueprintResources/StandardMacros.IncrementInt` (`self.CurrentWeaponMeleeIndex`)
      (:`  `
        (`BlueprintMapLibrary.Map_Add` (`self.AvailableWeaponsMelee`) (`self.CurrentWeaponMeleeIndex`) _value)
        (return (`self.CurrentWeaponMeleeIndex`))))
    (else
      (`KismetSystemLibrary.PrintString` "No weapons found (Weapon Melee List). Check the name or add the weapon to the list."))))

(fn `ChangeWeapon`
  (params (WeaponComponent :type "/Game/Interaction/Blueprints/Weapon/BP_Weapon Object Reference") (AvailableWeaponIndex :type Integer))
  (set `/Game/Interaction/Blueprints/Weapon/BP_Weapon.WeaponListIndex` AvailableWeaponIndex WeaponComponent)
  (`/Game/Interaction/Blueprints/Weapon/BP_Weapon.SetWeaponParam` WeaponComponent (`BlueprintMapLibrary.Map_Find` (`self.AvailableWeapons`) AvailableWeaponIndex)))

(fn `GetAvailableWeaponMelee`
  (params (AvailableWeaponIndex :type Integer))
  (returns (WeaponMelee :type "/Game/Interaction/Blueprints/Pawn/Player/Components/Struct_Player_Melee_Weapon Structure"))
  (return (`BlueprintMapLibrary.Map_Find` (`self.AvailableWeaponsMelee`) AvailableWeaponIndex)))

(fn `GetAvailableWeaponParam`
  (params (AvailableWeaponIndex :type Integer))
  (returns (WeaponStruct :type "/Game/Interaction/Blueprints/Weapon/Structures/Struct_W Structure"))
  (return (`BlueprintMapLibrary.Map_Find` (`self.AvailableWeapons`) AvailableWeaponIndex)))

(fn `GetBaseWeaponParam`
  (params (WeaponName :type String))
  (returns (WeaponStruct :type "/Game/Interaction/Blueprints/Weapon/Structures/Struct_W Structure"))
  (bind (_value _returnvalue) (`BlueprintMapLibrary.Map_Find` (`self.WeaponList`) WeaponName))
  (if _returnvalue
    (return _value)
    (else
      (`KismetSystemLibrary.PrintString` "(Get weapon param) No weapons found. Check the name or add the weapon to the list." true true (struct :`R` 1.0 :`A` 1.0) 4.0))))