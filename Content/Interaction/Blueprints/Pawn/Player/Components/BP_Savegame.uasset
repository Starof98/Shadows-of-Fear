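; BP_Savegame is a save game object that stores the player's weapons, health and inventory state.
; Three events, SaveWeapons, SaveHealth and SaveInventory, each copy their inputs into the object's variables, covering weapon lists and equipped indices, health and recovery settings, or ammo and quest items.
; Each event then immediately saves the whole object to the shared "PlayerParam" slot, with no loading logic in this graph.
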(event `SaveWeapons`
  (params (AvailableWeapons :type "Map of Integer to /Game/Interaction/Blueprints/Weapon/Structures/Struct_W Structure (by ref)") (AvailableWeaponsMelee :type "Map of Integer to /Game/Interaction/Blueprints/Pawn/Player/Components/Struct_Player_Melee_Weapon Structure (by ref)") (PrimaryEquipedIndex :type Integer) (SecondaryEquipedIndex :type Integer) (MeleeEquipedIndex :type Integer))
  (set `self.AvailableWeapons` AvailableWeapons)
  (set `self.AvailableWeaponsMelee` AvailableWeaponsMelee)
  (set `self.PrimaryEquipedIndex` PrimaryEquipedIndex)
  (set `self.SecondaryEquipedIndex` SecondaryEquipedIndex)
  (set `self.MeleeEquipedIndex` MeleeEquipedIndex)
  (`GameplayStatics.SaveGameToSlot` self "PlayerParam"))

(event `SaveHealth`
  (params (MaxHealth :type "Float (double-precision)") (Health :type "Float (double-precision)") (HealthRecoveryValue :type "Float (double-precision)") (HealthRecoveryTime :type "Float (double-precision)"))
  (set `self.MaxHealth` MaxHealth)
  (set `self.Health` Health)
  (set `self.HealthRecoveryValue` HealthRecoveryValue)
  (set `self.HealthRecoveryTime` HealthRecoveryTime)
  (`GameplayStatics.SaveGameToSlot` self "PlayerParam"))

(event `SaveInventory`
  (params (Ammo :type "Map of String to Integer (by ref)") (QuestItems :type "Map of String to Integer (by ref)"))
  (set `self.Ammo` Ammo)
  (set `self.QuestItems` QuestItems)
  (`GameplayStatics.SaveGameToSlot` self "PlayerParam"))